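; BPAC_MakeInteractive is a component that makes objects interactive for the first-person player character.
; Interaction and inventory-interaction events relay to dispatchers, leaving the response to whatever binds them.
; Being looked at pushes the object and interaction names to the character's HUD.
; AddToInventory adds an item to the character's inventory after a Contains check, while GetBasicData returns an empty name.
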(event EventInventoryInteraction
  (Default|CallOnInventoryInteraction))

(event EventLookingat
  (bind _asfirst_person_character (Utilities|Casting|CastToFirstPersonCharacter (Game|GetPlayerCharacter 0)))
  (Default|SetLookingatHUD _asfirst_person_character (Variables|Default|GetName) (Variables|Default|GetInteractionName)))

(event EventActivateInteraction
  (Default|CallOnInteraction))

(fn AddtoInventory
  (params (Item :type Actor%20Object%20Reference))
  (bind _asfirst_person_character (Utilities|Casting|CastToFirstPersonCharacter (Game|GetPlayerCharacter 0)))
  (if (not (Utilities|Array|ContainsItem (Variables|/Game/FirstPersonController/Blueprints/FirstPersonCharacter.FirstPersonCharacter_C|GetInventory _asfirst_person_character) 0))
    (Utilities|Array|Add (Variables|/Game/FirstPersonController/Blueprints/FirstPersonCharacter.FirstPersonCharacter_C|GetInventory _asfirst_person_character) Item)))

(fn GetBasicData
  (return "" 0))